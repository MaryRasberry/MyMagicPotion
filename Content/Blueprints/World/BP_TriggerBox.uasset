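; Trigger box that sends a solved state to ActorsToReact through ReactMessage when BP_Player enters or leaves it.
; Begin and end overlaps have separate enable flags and solved values, with DoOnceWithAfter limiting either to one firing when its Once setting passes IsValid.
; Solved starts as the inverse of BeginOverlapSolved, updates on each firing and is exposed through ReturnSolvedStatus.
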(event OnComponentBeginOverlap(Box)
  (params (OverlappedComponent :type Primitive%20Component%20Object%20Reference) (OtherActor :type Actor%20Object%20Reference) (OtherComp :type Primitive%20Component%20Object%20Reference) (OtherBodyIndex :type Integer) (bFromSweep :type Boolean) (SweepResult :type Hit%20Result%20Structure%20%28by%20ref%29))
  (if (and (== (Utilities|GetClass OtherActor) "/Game/Blueprints/Core/BP_Player.BP_Player_C") (Variables|BeginOverlap|GetUseBeginOverlap))
    (Variables|BeginOverlap|GetBeginOverlapOnce
      (:then
        (Utilities|DoOncewithAfter
          (:once
            _)))
      (:else
        _))
    (Class|BPIReact|React(Message) (Variables|Default|GetActorsToReact) (Variables|BeginOverlap|GetBeginOverlapSolved))
    (Variables|Default|SetSolved (Variables|BeginOverlap|GetBeginOverlapSolved))))

(event OnComponentEndOverlap(Box)
  (params (OverlappedComponent :type Primitive%20Component%20Object%20Reference) (OtherActor :type Actor%20Object%20Reference) (OtherComp :type Primitive%20Component%20Object%20Reference) (OtherBodyIndex :type Integer))
  (if (and (== (Utilities|GetClass OtherActor) "/Game/Blueprints/Core/BP_Player.BP_Player_C") (Variables|EndOverlap|GetUseEndOverlap))
    (Utilities|DoOncewithAfter
      (:once
        _)
      (:after
        (Variables|EndOverlap|GetEndOverlapOnce
          (:then)
          (:else
            _))))
    (Class|BPIReact|React(Message) (Variables|Default|GetActorsToReact) (Variables|EndOverlap|GetEndOverlapSolved))
    (Variables|Default|SetSolved (Variables|EndOverlap|GetEndOverlapSolved))))

(fn ConstructionScript
  (Variables|Default|SetSolved (not (Variables|BeginOverlap|GetBeginOverlapSolved))))

(fn ReturnSolvedStatus
  (return (Variables|Default|GetSolved)))