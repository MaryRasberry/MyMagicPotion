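; Pawn for a cooking station's close-up view, possessed when the player uses the station and released by interacting with that station again.
; A timeline blends camera and control rotation between the player's view and the station view, both ways.
; While possessed, a looping timer line-traces for Player.CookingInteract, and interact input calls BPI_Interact on other hit actors.
; The player's CanUseInput counter gates look and interact input during transitions.
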(event Custom|InteractCheck
  (bind _camera (Variables|Default|GetCamera))
  (bind _returnvalue (Transformation|GetWorldLocation _camera))
  (Variables|Default|GetIsPossessed
    (:then
      (bind (_outhit _returnvalue_2) (Collision|LineTraceByChannel _returnvalue (+ _returnvalue (* (Math|Vector|GetForwardVector _camera) (Variables|/Game/Blueprints/Core/BP_Player.BP_Player_C|GetInteractDistance (Variables|Default|GetPlayer)))) "TraceTypeQuery1" false 0 "None"))
      (Variables|Default|SetTraceReturn _returnvalue_2)
      (Variables|Default|SetTraceResult _outhit)
      (Default|CookingInteract (Variables|Default|GetPlayer) (Variables|Default|GetTraceReturn) (Variables|Default|GetTraceResult)))
    (:else)))

(event Custom|StationInteract
  (params (Player :type BP%20Player%20Object%20Reference) (ParentStation :type BP%20Cooking%20Station%20Object%20Reference))
  (Variables|Default|SetParentStation ParentStation)
  (bind _output_get (Variables|Default|SetPlayer Player))
  (Variables|Default|SetControlRotation (Pawn|GetControlRotation _output_get :!class /Script/Engine.Pawn))
  (Math|Integer|IncrementInt (Variables|/Game/Blueprints/Core/BP_Player.BP_Player_C|GetCanUseInput (Variables|Default|GetPlayer))
    (:%20%20
      (Variables|Default|SetStartTransform (Transformation|GetWorldTransform (Variables|/Game/Blueprints/Core/BP_Player.BP_Player_C|GetCamera (Variables|Default|GetPlayer))))
      (Pawn|Possess (Game|GetPlayerController 0) self)
      (Variables|Default|SetIsPossessed true)
      (Variables|/Game/Blueprints/Core/BP_Player.BP_Player_C|SetIsPossessed (Variables|Default|GetPlayer) false)
      (Pawn|SetControlRotation (Game|GetPlayerController 0) (Variables|Default|GetControlRotation))
      (Transformation|SetWorldTransform (Variables|Default|GetCamera) (Variables|Default|GetStartTransform) false true)
      (Audio|Components|Audio|Play (Variables|Default|GetMoveTimeline)))))

(event Input|EnhancedActionEvents|EnhancedInputActionIA_Interact
  (params (ActionValue :type Boolean) (ElapsedSeconds :type Float%20%28double-precision%29) (TriggeredSeconds :type Float%20%28double-precision%29) (InputAction :type Input%20Action%20Object%20Reference :default "/Game/Inputs/IA_Interact.IA_Interact"))
  (bind _traceresult (Variables|Default|GetTraceResult))
  (bind _hitactor (Collision|BreakHitResult _traceresult))
  (:Started
    (Utilities|HasInput
      (:true
        (Variables|Default|GetTraceReturn
          (:then
            (if (== _hitactor (Variables|Default|GetParentStation))
              (Math|Integer|IncrementInt (Variables|/Game/Blueprints/Core/BP_Player.BP_Player_C|GetCanUseInput (Variables|Default|GetPlayer))
                (:%20%20
                  (Variables|Default|SetLeaveTransform (Transformation|GetWorldTransform (Variables|Default|GetCamera)))
                  (Utilities|String|Reverse (Variables|Default|GetMoveTimeline))
                  (Collision|SetCollisionEnabled (Variables|/Game/Blueprints/World/BP_CookingStation.BP_CookingStation_C|GetBox (Variables|Default|GetParentStation)) "QueryOnly")))
              (elif (Utilities|DoesObjectImplementInterface _hitactor "/Game/Blueprints/Interfaces/BPI_Interact.BPI_Interact_C")
                (Default|CallInteract _hitactor (Variables|Default|GetPlayer) (Transformation|GetWorldTransform (Variables|Default|GetCamera))))))
          (:else))))))

(event Input|EnhancedActionEvents|EnhancedInputActionIA_Look
  (params (ActionValue :type Vector%202D%20Structure) (ElapsedSeconds :type Float%20%28double-precision%29) (TriggeredSeconds :type Float%20%28double-precision%29) (InputAction :type Input%20Action%20Object%20Reference :default "/Game/Inputs/IA_Look.IA_Look"))
  (bind (_x _y) (Math|Vector2D|BreakVector2D ActionValue))
  (Utilities|HasInput
    (:true
      (Pawn|Input|AddControllerYawInput _x)
      (Pawn|Input|AddControllerPitchInput _y))))

(event EventBeginPlay
  (Variables|Default|SetBaseTransform (Transformation|GetWorldTransform (Variables|Default|GetCamera)))
  (Components|Timeline|SetPlayRate (Variables|Default|GetMoveTimeline) (|(1/Seconds) (Variables|Default|GetMoveDuration)))
  (Utilities|Time|SetTimerbyFunctionName 0 "InteractCheck" 0.1 true true))

(event Collision|EventActorBeginOverlap
  (params (OtherActor :type Actor%20Object%20Reference)))

(event EventTick
  (params (DeltaSeconds :type Float%20%28single-precision%29)))

(fn ConstructionScript)