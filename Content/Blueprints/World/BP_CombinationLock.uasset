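; Interactable combination lock puzzle with three rotating dials that notifies linked actors when solved.
; Interacting smoothly possesses the lock and adds a lock widget; move input selects a highlighted dial or steps it through preset rotations, wrapping around.
; Each turn checks the current combination against the solution.
; Solving or pressing interact returns possession, control rotation and UI to the player, and a solved lock stops being interactable.
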(event Custom|UpAndDown
  (params (Y :type Float%20%28double-precision%29))
  (bind _currentcombination (Variables|Default|GetCurrentCombination))
  (bind _dialindex (Variables|Default|GetDialIndex))
  (bind _currentcombination_2 (Variables|Default|GetCurrentCombination))
  (bind _dialindex_2 (Variables|Default|GetDialIndex))
  (bind _output (Utilities|Array|Get(acopy) _currentcombination _dialindex))
  (bind _output_2 (Utilities|Array|Get(acopy) _currentcombination_2 _dialindex_2))
  (bind _returnvalue (+ _output 1))
  (bind _returnvalue_2 (- _output_2 1))
  (Math|Float|CompareFloat Y 0.0
    (:>
      (Utilities|Array|SetArrayElem (Variables|Default|GetCurrentCombination) (Variables|Default|GetDialIndex) (Math|Integer|SelectInt 0 _returnvalue (> _returnvalue (Utilities|Array|LastIndex (Variables|Default|GetRotationPoints)))))
      (CallFunction|RotateDial))
    (:<
      (Utilities|Array|SetArrayElem (Variables|Default|GetCurrentCombination) (Variables|Default|GetDialIndex) (Math|Integer|SelectInt (Utilities|Array|LastIndex (Variables|Default|GetRotationPoints)) _returnvalue_2 (< _returnvalue_2 0)))
      (CallFunction|RotateDial))))

(event Custom|LeftAndRight
  (params (X :type Float%20%28double-precision%29))
  (Math|Float|CompareFloat X 0.0
    (:>
      (Variables|Default|SetDialIndex (Math|Integer|SelectInt 0 (+ (Variables|Default|GetDialIndex) 1) (> (+ (Variables|Default|GetDialIndex) 1) (Utilities|Array|LastIndex (Variables|Default|GetDials)))))
      (CallFunction|HighlightDial))
    (:<
      (Variables|Default|SetDialIndex (Math|Integer|SelectInt (Utilities|Array|LastIndex (Variables|Default|GetDials)) (- (Variables|Default|GetDialIndex) 1) (< (- (Variables|Default|GetDialIndex) 1) 0)))
      (CallFunction|HighlightDial))))

(event Custom|RotateDial
  (Transformation|SetRelativeRotation (Utilities|Array|Get(acopy) (Variables|Default|GetDials) (Variables|Default|GetDialIndex)) (Utilities|Array|Get(acopy) (Variables|Default|GetRotationPoints) (Utilities|Array|Get(acopy) (Variables|Default|GetCurrentCombination) (Variables|Default|GetDialIndex))) false false)
  (bind _solved (CallFunction|ReturnSolvedStatus))
  (if _solved
    (Variables|Default|SetSolved true)
    (CallFunction|LeaveLock)))

(event Custom|LeaveLock
  (Variables|Default|GetHasInput
    (:then
      (Variables|Default|SetHasInput false)
      (Math|Integer|DecrementInt (Variables|/Game/Blueprints/Core/BP_Player.BP_Player_C|GetCanUseInput (Variables|Default|GetPlayerRef))
        (:%20%20
          (Utilities|SmoothPossess (Game|GetPlayerController 0) (Variables|Default|GetPlayerRef) 1.0)
          (Rendering|Material|SetOverlayMaterial (Variables|Default|GetDials) 0 :!class /Script/Engine.MeshComponent)
          (Pawn|SetControlRotation (Game|GetPlayerController 0) (Variables|Default|GetControlRotation))
          (Class|CommonActivatableWidgetContainerBase|RemoveWidget (CallFunction|ReturnMainStack (Game|GetPlayerController 0)) (Variables|Default|GetWidget))
          (Variables|Default|GetSolved
            (:then
              (Class|BPIReact|React(Message) (Variables|Default|GetActorsToRect) true))
            (:else)))))
    (:else)))

(event Input|EnhancedActionEvents|EnhancedInputActionIA_Interact
  (params (ActionValue :type Boolean) (ElapsedSeconds :type Float%20%28double-precision%29) (TriggeredSeconds :type Float%20%28double-precision%29) (InputAction :type Input%20Action%20Object%20Reference :default "/Game/Inputs/IA_Interact.IA_Interact"))
  (:Started
    (CallFunction|LeaveLock)))

(event Input|EnhancedActionEvents|EnhancedInputActionIA_Move
  (params (ActionValue :type Vector%202D%20Structure) (ElapsedSeconds :type Float%20%28double-precision%29) (TriggeredSeconds :type Float%20%28double-precision%29) (InputAction :type Input%20Action%20Object%20Reference :default "/Game/Inputs/IA_Move.IA_Move"))
  (bind (_x _y) (Math|Vector2D|BreakVector2D ActionValue))
  (:Started
    (Variables|Default|GetHasInput
      (:then
        (Variables|Default|GetSolved
          (:then)
          (:else
            (Math|Float|CompareFloat (Math|Float|Absolute(Float) _x) (Math|Float|Absolute(Float) _y)
              (:>
                (CallFunction|LeftandRight _x))
              (:<
                (CallFunction|UpandDown _y))))))
      (:else))))

(event EventBeginPlay
  (Variables|Default|SetDials (Utilities|Array|MakeArray (Variables|Default|Get00) (Variables|Default|Get01) (Variables|Default|Get02))))

(event EventInteract
  (params (Player :type BP%20Player%20Object%20Reference))
  (bind _output_get (Variables|Default|SetPlayerRef Player))
  (Math|Integer|IncrementInt (Variables|/Game/Blueprints/Core/BP_Player.BP_Player_C|GetCanUseInput _output_get)
    (:%20%20
      (Variables|Default|SetControlRotation (Pawn|GetControlRotation (Variables|Default|GetPlayerRef) :!class /Script/Engine.Pawn))
      (Utilities|SmoothPossess (Game|GetPlayerController 0) self 1.0)
      (CallFunction|HighlightDial)
      (bind _returnvalue (Class|CommonActivatableWidgetContainerBase|AddWidget (CallFunction|ReturnMainStack (Game|GetPlayerController 0)) "/Game/Blueprints/UI/CAW_Lock.CAW_Lock_C"))
      (Variables|Default|SetWidget _returnvalue)
      (Variables|Default|SetHasInput true))))

(fn ConstructionScript)

(fn HighlightDial
  (for (_array_element _array_index) (Variables|Default|GetDials)
    (if (== _array_index (Variables|Default|GetDialIndex))
      (Rendering|Material|SetOverlayMaterial _array_element "/Game/Materials/World/GameMaterials/MI_Highlight.MI_Highlight" :!class /Script/Engine.MeshComponent)
      (else
        (Rendering|Material|SetOverlayMaterial _array_element 0 :!class /Script/Engine.MeshComponent)))))

(fn ReturnInteractStatus
  (return (and (Variables|Default|GetIsInteractable) (not (Variables|Default|GetSolved))) "NewEnumerator6"))

(fn ReturnSolvedStatus
  (bind (_array_element _array_index) (Utilities|Array|ForEachLoopwithBreak (Variables|Default|GetCurrentCombination) :!label _label)
    (:LoopBody
      (if (!= _array_element (Utilities|Array|Get(acopy) (Variables|Default|GetSolvedCombination) _array_index))
        (LocalVariables|SetIsSolved false)
        (goto _label Break)))
    (:Completed
      (return (or (LocalVariables|GetIsSolved) (Variables|Default|GetSolved))))))