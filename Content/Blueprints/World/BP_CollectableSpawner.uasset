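; BP_CollectableSpawner is a world actor that spawns a configurable collectable at its own transform when it reacts to a solved state.
; React spawns only if no current collectable is valid, then binds to the new one's collected event.
; On collection it unbinds and clears the reference, allowing a later respawn.
; Its own ReturnSolvedStatus always reports false.
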(event Custom|CurrentCollectableCollected
  (EventDispatchers|UnbindEventfromOnCollected (Variables|Default|GetCurrentCollectable) (EventDispatchers|CreateEvent :!event Custom|CurrentCollectableCollected))
  (Variables|Default|SetCurrentCollectable 0))

(event EventReact
  (params (Solved :type Boolean))
  (if Solved
    (Variables|Default|GetCurrentCollectable
      (:then)
      (:else
        (bind _returnvalue (Game|SpawnActorfromClass (Variables|Default|GetCollectableToSpawn) (Transformation|GetActorTransform) "AdjustIfPossibleButAlwaysSpawn" "MultiplyWithRoot" 0 0))
        (bind _output_get (Variables|Default|SetCurrentCollectable _returnvalue))
        (EventDispatchers|BindEventtoOnCollected _output_get (EventDispatchers|CreateEvent :!event Custom|CurrentCollectableCollected))))))

(fn ConstructionScript)

(fn ReturnSolvedStatus
  (return false))