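; BP_GuidingParticle is a world actor that sends a Niagara particle along a spline as a guide for the player.
; It starts on BeginPlay when AutoPlay passes its check, or once when React receives a solved state.
; A timeline, with play rate derived from Speed, is set up to lerp the effect along the spline's length.
; The player overlapping EndTrigger during playback stops the timeline and deactivates the effect.
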(event OnComponentBeginOverlap(EndTrigger)
  (params (OverlappedComponent :type Primitive%20Component%20Object%20Reference) (OtherActor :type Actor%20Object%20Reference) (OtherComp :type Primitive%20Component%20Object%20Reference) (OtherBodyIndex :type Integer) (bFromSweep :type Boolean) (SweepResult :type Hit%20Result%20Structure%20%28by%20ref%29))
  (if (== (Utilities|GetClass OtherActor) "/Game/Blueprints/Core/BP_Player.BP_Player_C")
    (if (Audio|Components|Audio|IsPlaying (Variables|Default|GetParticleTimeline))
      (Utilities|DoOncewithAfter
        (:once
          (Components|Activation|Deactivate (Variables|Default|GetNS_GuidingParticle))
          (Audio|Components|Audio|Stop (Variables|Default|GetParticleTimeline)))))))

(event Custom|StartGuidingParticle
  (Audio|Components|Audio|Play (Variables|Default|GetParticleTimeline))
  (Components|Activation|Activate (Variables|Default|GetNS_GuidingParticle) false))

(event EventBeginPlay
  (Components|Timeline|SetPlayRate (Variables|Default|GetParticleTimeline) (|SpeedToPlayrate (Variables|Default|GetSpeed)))
  (Variables|Default|GetAutoPlay
    (:then
      (CallFunction|StartGuidingParticle))
    (:else)))

(event EventReact
  (params (Solved :type Boolean))
  (if Solved
    (Utilities|DoOncewithAfter
      (:once
        (CallFunction|StartGuidingParticle)))))

(fn ConstructionScript)

(fn ReturnSolvedStatus
  (return false))