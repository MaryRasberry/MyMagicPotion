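; BP_Spotlight2 is a non-interactable puzzle-response light that brightens when triggered.
; Its React event plays a positive puzzle sound, then sets spotlight and point light intensities from variables, each gated by its own reference validity check.
; Status functions report it as not interactable and return a Solved flag, which these graphs never set.
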(event EventReact
  (params (Solved :type Boolean))
  (Audio|PlaySound2D "/Game/Audio/SoundSources/PuzzlePositive.PuzzlePositive" 1.0 1.0 0.0 0 0)
  (Utilities|FlowControl|Sequence
    (:then_0
      (Variables|Spotlight|GetAcitvateSpotlight
        (:then
          (Rendering|Components|Light|SetIntensity (Variables|Default|GetSpotLight) (Variables|Spotlight|GetSpotlightIntens)))
        (:else)))
    (:then_1
      (Variables|Pointlight|GetActivatePointlight
        (:then
          (Rendering|Components|Light|SetIntensity (Variables|Default|GetPointLight) (Variables|Pointlight|GetPointLightIntens)))
        (:else)))))

(fn ConstructionScript)

(fn ReturnInteractStatus
  (return false "NewEnumerator0"))

(fn ReturnSolvedStatus
  (return (Variables|Default|GetSolved)))