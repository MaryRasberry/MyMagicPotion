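; BP_Moveable is an interactable world object that toggles a scene component between its starting transform and a target transform.
; Interact runs a key check, optionally destroying the key, and plays a positive or negative puzzle sound.
; A correct key, or a React call that skips the check, advances a FlipFlop choosing the destination for an eased, timed MoveComponentTo.
; It reports its interact status and always returns unsolved.
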(event Custom|Move
  (params (Transform :type Transform%20%28by%20ref%29))
  (bind (_location _rotation) (Math|Transform|BreakTransform Transform))
  (Components|MoveComponentTo (Variables|Default|GetMoveScene) _location _rotation true true (Variables|Default|GetMoveDuration) true))

(event EventReact
  (params (Solved :type Boolean))
  (bind _isa (Utilities|FlowControl|FlipFlop)
    (:A
      _)
    (:B
      _))
  (CallFunction|Move (Math|Transform|SelectTransform (Variables|Default|GetTargetTransform) (Variables|Default|GetStartTransform) _isa)))

(event EventInteract
  (params (Player :type BP%20Player%20Object%20Reference))
  (Utilities|CheckforKey Player (Variables|Default|GetNeededKey) (Variables|Default|GetDestroyKey)
    (:CorrectKey
      (Audio|PlaySound2D "/Game/Audio/SoundSources/PuzzlePositive.PuzzlePositive" 1.0 1.0 0.0 0 0)
      (bind _isa (Utilities|FlowControl|FlipFlop)
        (:A
          _)
        (:B
          _))
      (CallFunction|Move (Math|Transform|SelectTransform (Variables|Default|GetTargetTransform) (Variables|Default|GetStartTransform) _isa)))
    (:WrongKey
      (Audio|PlaySound2D "/Game/Audio/SoundSources/PuzzleNegativeSound.PuzzleNegativeSound" 1.0 1.0 0.0 0 0))))

(event EventBeginPlay
  (Variables|Default|SetStartTransform (Transformation|GetRelativeTransform (Variables|Default|GetMoveScene))))

(fn ConstructionScript)

(fn ReturnInteractStatus
  (return (Variables|Default|GetIsInteractable) "NewEnumerator2"))

(fn ReturnSolvedStatus
  (return false))