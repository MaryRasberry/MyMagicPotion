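; BP_MagicBook is an interactable, possessable book the player uses to browse recipes.
; Possess moves its camera to a given transform, takes player control and pushes the book widget onto the main UI stack, applying the starting recipe only the first time.
; Move input flips recipes up to an unlockable maximum index, and Interact closes the widget and signals possession lost.
; New-recipe events from the widget are relayed through the book's own call.
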(event Custom|Possess
  (params (CameraTransform :type Transform))
  (Variables|Default|SetControlRotation (.Rotation (Math|Transform|BreakTransform CameraTransform)))
  (Transformation|SetWorldTransform (Variables|Default|GetCamera) CameraTransform false true)
  (Pawn|Possess (Game|GetPlayerController 0) self)
  (bind _returnvalue (Class|CommonActivatableWidgetContainerBase|AddWidget (CallFunction|ReturnMainStack (Game|GetPlayerController 0)) "/Game/Blueprints/UI/CAW_MagicBook.CAW_MagicBook_C"))
  (bind _output_get (Variables|Default|SetWidget _returnvalue))
  (Utilities|DoOncewithAfter
    (:once
      (Default|StartingRecipe _output_get (Variables|Default|GetStartinRecipeIndex)))
    (:after
      _))
  (EventDispatchers|BindEventtoNewRecipe _output_get (EventDispatchers|CreateEvent :!event Custom|NewRecipe)))

(event Custom|NewRecipe
  (params (RecipeIndex :type Integer))
  (Default|CallNewRecipetoUse RecipeIndex))

(event Custom|StartingRecepi
  (params (RecipeIndex :type Integer))
  (Variables|Default|SetStartinRecipeIndex RecipeIndex))

(event Custom|IncreaseRecepiLimit
  (Math|Integer|IncrementInt (Variables|Default|GetMaxRecepiIndex)))

(event Input|EnhancedActionEvents|EnhancedInputActionIA_Interact
  (params (ActionValue :type Boolean) (ElapsedSeconds :type Float%20%28double-precision%29) (TriggeredSeconds :type Float%20%28double-precision%29) (InputAction :type Input%20Action%20Object%20Reference :default "/Game/Inputs/IA_Interact.IA_Interact"))
  (:Started
    (Class|CommonActivatableWidgetContainerBase|RemoveWidget (CallFunction|ReturnMainStack (Game|GetPlayerController 0)) (Variables|Default|GetWidget))
    (EventDispatchers|UnbindEventfromNewRecipe (Variables|Default|GetWidget) (EventDispatchers|CreateEvent :!event Custom|NewRecipe))
    (Variables|Default|SetWidget 0)
    (Default|CallPossessionLost)))

(event Input|EnhancedActionEvents|EnhancedInputActionIA_Move
  (params (ActionValue :type Vector%202D%20Structure) (ElapsedSeconds :type Float%20%28double-precision%29) (TriggeredSeconds :type Float%20%28double-precision%29) (InputAction :type Input%20Action%20Object%20Reference :default "/Game/Inputs/IA_Move.IA_Move"))
  (bind _widget (Variables|Default|GetWidget))
  (:Started
    (Variables|Default|GetWidget
      (:then
        (Math|Float|CompareFloat (.X (Math|Vector2D|BreakVector2D ActionValue)) 0.0
          (:>
            (if (< (Class|CommonVisibilitySwitcher|GetActiveWidgetIndex (Variables|/Game/Blueprints/UI/CAW_MagicBook.CAW_MagicBook_C|GetSwitcherRecipi _widget)) (Variables|Default|GetMaxRecepiIndex))
              (Default|IncrementSwitcher _widget)))
          (:<
            (Default|DecrementSwitcher _widget))))
      (:else))))

(fn ConstructionScript)

(fn ReturnInteractStatus
  (return (Variables|Default|GetIsInteractable) "NewEnumerator8"))