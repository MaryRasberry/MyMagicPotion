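; BP_CutsceneManager plays an assigned level sequence when it receives a solved React message, then relays that message to ActorsToReact.
; During playback it adds a cutscene widget to the main stack and increments the player's CanUseInput counter, undoing both on finish.
; The relay waits ReactDelay after playback starts, or fires immediately without a sequence.
; PlayOnce limits this to one trigger; later or unsolved triggers relay false.
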(event Custom|OnFinished
  (Utilities|FlowControl|Sequence
    (:then_0
      (bind _playerref (Variables|Default|GetPlayerRef)
        (:then
          (Math|Integer|DecrementInt (Variables|/Game/Blueprints/Core/BP_Player.BP_Player_C|GetCanUseInput _playerref)))
        (:else)))
    (:then_1
      (Class|CommonActivatableWidgetContainerBase|RemoveWidget (CallFunction|ReturnMainStack (Game|GetPlayerController 0)) (Variables|Default|GetWidget)))))

(event EventReact
  (params (Solved :type Boolean))
  (if Solved
    (Variables|Default|GetPlayOnce
      (:then
        (Utilities|DoOncewithAfter
          (:once
            (bind _cutscenetoplay (Variables|Default|GetCutsceneToPlay :!label _label)
              (:then
                (Utilities|FlowControl|Sequence
                  (:then_0
                    (Utilities|FlowControl|Sequence
                      (:then_0
                        (bind _returnvalue (Class|CommonActivatableWidgetContainerBase|AddWidget (CallFunction|ReturnMainStack (Game|GetPlayerController 0)) "/Game/Blueprints/UI/CAW_Cutscene.CAW_Cutscene_C"))
                        (Variables|Default|SetWidget _returnvalue)
                        (Variables|Default|GetPlayerRef
                          (:then
                            _)
                          (:else
                            (bind _asbp_player (Utilities|Casting|CastToBP_Player (Game|GetPlayerCharacter 0)))
                            (Variables|Default|SetPlayerRef _asbp_player)))
                        (Math|Integer|IncrementInt (Variables|/Game/Blueprints/Core/BP_Player.BP_Player_C|GetCanUseInput (Variables|Default|GetPlayerRef))))
                      (:then_1
                        (EventDispatchers|BindEventtoOnFinished (Variables|/Script/LevelSequence.LevelSequenceActor|GetSequencePlayer _cutscenetoplay) (EventDispatchers|CreateEvent :!event Custom|OnFinished)))
                      (:then_2
                        (Sequencer|Player|Play (Variables|/Script/LevelSequence.LevelSequenceActor|GetSequencePlayer _cutscenetoplay) :!class /Script/MovieScene.MovieSceneSequencePlayer))))
                  (:then_1
                    (Utilities|FlowControl|Delay (Variables|Default|GetReactDelay))
                    (Class|BPIReact|React(Message) (Variables|Default|GetActorsToReact) true))))
              (:else
                (Class|BPIReact|React(Message) (Variables|Default|GetActorsToReact) true))))
          (:after
            (Class|BPIReact|React(Message) (Variables|Default|GetActorsToReact) false))))
      (:else
        (goto _label)))
    (else
      (Class|BPIReact|React(Message) (Variables|Default|GetActorsToReact) false))))

(fn ConstructionScript)

(fn ReturnSolvedStatus
  (return false))