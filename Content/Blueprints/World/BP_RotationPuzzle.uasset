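; Interactable world puzzle piece that the player rotates through preset orientations, notifying linked actors when it reaches or leaves its solved position.
; Interaction passes a key check, then advances a wrapping index and eases the Scene component to that rotation.
; Matching the solved index sends a true react message to ActorsToReact, while a DoOnce limits the false message to once per solve.
; The construction script applies the starting rotation.
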(event EventSetInteractStatus
  (params (NewInteractStatus :type Boolean))
  (Variables|Default|SetIsInteractable NewInteractStatus))

(event EventInteract
  (params (Player :type BP%20Player%20Object%20Reference))
  (Utilities|CheckforKey Player (Variables|Default|GetNeededKey) (Variables|Default|GetDestroyKey)
    (:CorrectKey
      (Variables|Default|SetCurrentRotationIndex (Math|Integer|SelectInt (+ (Variables|Default|GetCurrentRotationIndex) 1) 0 (< (+ (Variables|Default|GetCurrentRotationIndex) 1) (Utilities|Array|Length (Variables|Default|GetRotationPoints)))))
      (Components|MoveComponentTo (Variables|Default|GetScene) "0, 0, 0" (Utilities|Array|Get(acopy) (Variables|Default|GetRotationPoints) (Variables|Default|GetCurrentRotationIndex)) true true 0.2 true)
      (bind _solved (CallFunction|ReturnSolvedStatus))
      (if _solved
        (Class|BPIReact|React(Message) (Variables|Default|GetActorsToReact) true)
        (goto _label Reset)
        (else
          (Utilities|FlowControl|DoOnce true :!label _label
            (:Completed
              (Class|BPIReact|React(Message) (Variables|Default|GetActorsToReact) false))))))))

(fn ConstructionScript
  (Transformation|SetRelativeRotation (Variables|Default|GetScene) (Utilities|Array|Get(acopy) (Variables|Default|GetRotationPoints) (Variables|Default|GetCurrentRotationIndex)) false false))

(fn ReturnInteractStatus
  (return (Variables|Default|GetIsInteractable) "NewEnumerator4"))

(fn ReturnSolvedStatus
  (return (== (Variables|Default|GetCurrentRotationIndex) (Variables|Default|GetSolvedIndex))))