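; Interactable Simon Says puzzle pawn that the player smooth-possesses, navigating a 2x2 button grid and pressing Jump to repeat a sequence.
; With a TargetLength, it grows a random sequence and plays it through emissive dynamic materials; otherwise it checks preset CorrectRows/CorrectColumns.
; Overlay material marks selection; mistakes flash all buttons wrong and restart progress.
; Solving or cancelling returns possession and removes the widget, with solving also notifying ActorsToRect.
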(event Custom|LeaveSimonSays
  (Variables|Default|GetHasInput
    (:then
      (Variables|Default|SetHasInput false)
      (Math|Integer|DecrementInt (Variables|/Game/Blueprints/Core/BP_Player.BP_Player_C|GetCanUseInput (Variables|Default|GetPlayerRef))
        (:%20%20
          (Utilities|SmoothPossess (Game|GetPlayerController 0) (Variables|Default|GetPlayerRef) 1.0)
          (CallFunction|HighlightButton false)
          (Pawn|SetControlRotation (Game|GetPlayerController 0) (Variables|Default|GetControlRotation))
          (Class|CommonActivatableWidgetContainerBase|RemoveWidget (CallFunction|ReturnMainStack (Game|GetPlayerController 0)) (Variables|Default|GetWidget))
          (Variables|Default|GetSolved
            (:then
              (Class|BPIReact|React(Message) (Variables|Default|GetActorsToRect) true))
            (:else)))))
    (:else)))

(event Custom|LeftAndRight
  (params (Input :type Float%20%28double-precision%29))
  (Math|Float|CompareFloat Input 0.0
    (:>
      (Variables|Default|SetCurrentColumn (Math|Integer|SelectInt 0 (+ (Variables|Default|GetCurrentColumn) 1) (> (+ (Variables|Default|GetCurrentColumn) 1) (Utilities|Array|LastIndex (Utilities|Struct|BreakSt_SimonSaysRow (Utilities|Array|Get(acopy) (Variables|Default|GetButtons) (Variables|Default|GetCurrentRow)))))))
      (CallFunction|HighlightButton true))
    (:<
      (Variables|Default|SetCurrentColumn (Math|Integer|SelectInt (Utilities|Array|LastIndex (Utilities|Struct|BreakSt_SimonSaysRow (Utilities|Array|Get(acopy) (Variables|Default|GetButtons) (Variables|Default|GetCurrentRow)))) (- (Variables|Default|GetCurrentColumn) 1) (< (- (Variables|Default|GetCurrentColumn) 1) 0)))
      (CallFunction|HighlightButton true))))

(event Custom|UpAndDown
  (params (Input :type Float%20%28double-precision%29))
  (Math|Float|CompareFloat Input 0.0
    (:>
      (Variables|Default|SetCurrentRow (Math|Integer|SelectInt (Utilities|Array|LastIndex (Variables|Default|GetButtons)) (- (Variables|Default|GetCurrentRow) 1) (< (- (Variables|Default|GetCurrentRow) 1) 0)))
      (CallFunction|HighlightButton true))
    (:<
      (Variables|Default|SetCurrentRow (Math|Integer|SelectInt 0 (+ (Variables|Default|GetCurrentRow) 1) (> (+ (Variables|Default|GetCurrentRow) 1) (Utilities|Array|LastIndex (Variables|Default|GetButtons)))))
      (CallFunction|HighlightButton true))))

(event Custom|DisplayTargetButtons
  (bind _buttons (Variables|Default|GetButtons))
  (bind (_outitem _outindex) (Utilities|Array|Random _buttons))
  (Variables|Default|SetHasInput false)
  (if (< (Variables|Default|GetCurrentLength) (Variables|Default|GetTargetLength))
    (Variables|Default|SetProgress 0)
    (bind _result (Math|Integer|IncrementInt (Variables|Default|GetCurrentLength))
      (:%20%20
        (if (== _result 1)
          (Utilities|Array|Clear (Variables|Default|GetCorrectRows))
          (Utilities|Array|Clear (Variables|Default|GetCorrectColumns)))
        (Utilities|Array|Add (Variables|Default|GetCorrectRows) (.OutIndex (Utilities|Array|Random (Utilities|Struct|BreakSt_SimonSaysRow _outitem))))
        (Utilities|Array|Add (Variables|Default|GetCorrectColumns) _outindex)
        (bind _index (Utilities|ForLoopwithDelay 0 (Utilities|Array|LastIndex (Variables|Default|GetCorrectRows)) :!label _label)
          (:LoopBody
            (Rendering|Material|SetScalarParameterValue (Utilities|Array|Get(acopy) (Utilities|Struct|BreakSt_SimonSaysRow (Utilities|Array|Get(acopy) (Variables|Default|GetButtons) (Utilities|Array|Get(acopy) (Variables|Default|GetCorrectRows) _index))) (Utilities|Array|Get(acopy) (Variables|Default|GetCorrectColumns) _index)) "Emissive" 1.0 :!class /Script/Engine.MaterialInstanceDynamic)
            (Utilities|FlowControl|Delay 0.5)
            (Rendering|Material|SetScalarParameterValue (Utilities|Array|Get(acopy) (Utilities|Struct|BreakSt_SimonSaysRow (Utilities|Array|Get(acopy) (Variables|Default|GetButtons) (Utilities|Array|Get(acopy) (Variables|Default|GetCorrectRows) _index))) (Utilities|Array|Get(acopy) (Variables|Default|GetCorrectColumns) _index)) "Emissive" 0.1 :!class /Script/Engine.MaterialInstanceDynamic))
          (:Completed
            (Variables|Default|SetHasInput true))
          (:OutDelay
            (Utilities|FlowControl|Delay 0.6)
            (goto _label InDelay)))))
    (else
      (Variables|Default|SetHasInput true))))

(event Custom|ShowFeedback
  (params (Correct :type Boolean))
  (if Correct
    (Variables|Default|SetCanProgress false)
    (bind _output_get (Variables|Default|SetCurrentHighlightedMaterial (Utilities|Array|Get(acopy) (Utilities|Struct|BreakSt_SimonSaysRow (Utilities|Array|Get(acopy) (Variables|Default|GetButtons) (Variables|Default|GetCurrentRow))) (Variables|Default|GetCurrentColumn))))
    (Rendering|Material|SetScalarParameterValue _output_get "Emissive" 2.0 :!class /Script/Engine.MaterialInstanceDynamic)
    (Utilities|FlowControl|Delay 0.2)
    (Rendering|Material|SetScalarParameterValue (Variables|Default|GetCurrentHighlightedMaterial) "Emissive" 0.1 :!class /Script/Engine.MaterialInstanceDynamic)
    (if (and (>= (Variables|Default|GetProgress) (Variables|Default|GetCurrentLength)) (< (Variables|Default|GetProgress) (Variables|Default|GetTargetLength)))
      (Utilities|FlowControl|Delay 1.0)
      (CallFunction|DisplayTargetButtons)
      (Variables|Default|SetCanProgress true)
      (else
        (Variables|Default|SetCanProgress true)))
    (else
      (Variables|Default|SetHasInput false)
      (for _array_element (Variables|Default|GetButtons)
        (Rendering|Material|SetMaterial (Utilities|Struct|BreakSt_SimonSaysRow _array_element) 0 "/Game/Materials/World/GameMaterials/MI_SimonSaysWrong.MI_SimonSaysWrong"))
      (Utilities|FlowControl|Delay 1.0)
      (for _array_element_2 (Variables|Default|GetButtons)
        (for (_array_element_3 _array_index) (.Meshes (Utilities|Struct|BreakSt_SimonSaysRow _array_element_2))
          (Rendering|Material|SetMaterial _array_element_3 0 (Utilities|Array|Get(acopy) (.Materials (Utilities|Struct|BreakSt_SimonSaysRow _array_element_2)) _array_index))
          (Variables|Default|SetCanProgress true)))
      (if (Math|Conversions|ToBoolean(Integer) (Variables|Default|GetTargetLength))
        (Utilities|FlowControl|Delay 1.0)
        (Variables|Default|SetCurrentLength 0)
        (CallFunction|DisplayTargetButtons)
        (else
          (Variables|Default|SetHasInput true))))))

(event Input|EnhancedActionEvents|EnhancedInputActionIA_Interact
  (params (ActionValue :type Boolean) (ElapsedSeconds :type Float%20%28double-precision%29) (TriggeredSeconds :type Float%20%28double-precision%29) (InputAction :type Input%20Action%20Object%20Reference :default "/Game/Inputs/IA_Interact.IA_Interact"))
  (CallFunction|LeaveSimonSays))

(event Input|EnhancedActionEvents|EnhancedInputActionIA_Move
  (params (ActionValue :type Vector%202D%20Structure) (ElapsedSeconds :type Float%20%28double-precision%29) (TriggeredSeconds :type Float%20%28double-precision%29) (InputAction :type Input%20Action%20Object%20Reference :default "/Game/Inputs/IA_Move.IA_Move"))
  (bind (_x _y) (Math|Vector2D|BreakVector2D ActionValue))
  (:Started
    (Variables|Default|GetHasInput
      (:then
        (Variables|Default|GetSolved
          (:then)
          (:else
            (Math|Float|CompareFloat (Math|Float|Absolute(Float) _x) (Math|Float|Absolute(Float) _y)
              (:>
                (CallFunction|LeftandRight _x))
              (:<
                (CallFunction|UpandDown _y))))))
      (:else))))

(event Input|EnhancedActionEvents|EnhancedInputActionIA_Jump
  (params (ActionValue :type Boolean) (ElapsedSeconds :type Float%20%28double-precision%29) (TriggeredSeconds :type Float%20%28double-precision%29) (InputAction :type Input%20Action%20Object%20Reference :default "/Game/Inputs/IA_Jump.IA_Jump"))
  (:Started
    (if (Math|Boolean|ANDBoolean (not (Variables|Default|GetSolved)) (Variables|Default|GetCanProgress) (Variables|Default|GetHasInput))
      (if (and (== (Variables|Default|GetCurrentRow) (Utilities|Array|Get(acopy) (Variables|Default|GetCorrectRows) (Variables|Default|GetProgress))) (== (Variables|Default|GetCurrentColumn) (Utilities|Array|Get(acopy) (Variables|Default|GetCorrectColumns) (Variables|Default|GetProgress))))
        (CallFunction|ShowFeedback true)
        (bind _result (Math|Integer|IncrementInt (Variables|Default|GetProgress))
          (:%20%20
            (if (> _result (Utilities|Array|LastIndex (Variables|Default|GetCorrectRows)))
              (if (>= (Variables|Default|GetProgress) (Variables|Default|GetTargetLength))
                (Variables|Default|SetSolved true)
                (CallFunction|LeaveSimonSays)))))
        (else
          (Variables|Default|SetProgress 0)
          (CallFunction|ShowFeedback false))))))

(event EventBeginPlay)

(event EventInteract
  (params (Player :type BP%20Player%20Object%20Reference))
  (bind _output_get (Variables|Default|SetPlayerRef Player))
  (Math|Integer|IncrementInt (Variables|/Game/Blueprints/Core/BP_Player.BP_Player_C|GetCanUseInput _output_get)
    (:%20%20
      (Variables|Default|SetControlRotation (Pawn|GetControlRotation (Variables|Default|GetPlayerRef) :!class /Script/Engine.Pawn))
      (Utilities|SmoothPossess (Game|GetPlayerController 0) self 1.0)
      (CallFunction|HighlightButton true)
      (bind _returnvalue (Class|CommonActivatableWidgetContainerBase|AddWidget (CallFunction|ReturnMainStack (Game|GetPlayerController 0)) "/Game/Blueprints/UI/CAW_SimonSays.CAW_SimonSays_C"))
      (Variables|Default|SetWidget _returnvalue)
      (if (Math|Conversions|ToBoolean(Integer) (Variables|Default|GetTargetLength))
        (Utilities|DoOncewithAfter
          (:once
            (CallFunction|DisplayTargetButtons))
          (:after
            (Variables|Default|SetHasInput true :!label _label)))
        (else
          (goto _label))))))

(fn ConstructionScript
  (bind _output_get (Variables|Default|SetButtons (Utilities|Array|MakeArray (Utilities|Struct|MakeSt_SimonSaysRow (Utilities|Array|MakeArray (Variables|Default|GetR101) (Variables|Default|GetR102))) (Utilities|Struct|MakeSt_SimonSaysRow (Utilities|Array|MakeArray (Variables|Default|GetR201) (Variables|Default|GetR202))))))
  (for (_array_element _array_index) _output_get
    (for (_array_element_2 _array_index_2) (Utilities|Struct|BreakSt_SimonSaysRow _array_element)
      (bind _returnvalue (Rendering|Material|CreateDynamicMaterialInstance _array_element_2 0 (Rendering|Material|GetMaterial _array_element_2 0) "None" :!class /Script/Engine.PrimitiveComponent))
      (Utilities|Array|SetArrayElem (Utilities|Struct|BreakSt_SimonSaysRow (Utilities|Array|Get(acopy) (Variables|Default|GetButtons) _array_index)) _array_index_2 _returnvalue true))))

(fn HighlightButton
  (params (EnableHighlight :type Boolean))
  (for _array_element (Variables|Default|GetButtons)
    (for _array_element_2 (Utilities|Struct|BreakSt_SimonSaysRow _array_element)
      (Rendering|Material|SetOverlayMaterial _array_element_2 0 :!class /Script/Engine.MeshComponent)))
  (if EnableHighlight
    (Rendering|Material|SetOverlayMaterial (Utilities|Array|Get(acopy) (Utilities|Struct|BreakSt_SimonSaysRow (Utilities|Array|Get(acopy) (Variables|Default|GetButtons) (Variables|Default|GetCurrentRow))) (Variables|Default|GetCurrentColumn)) "/Game/Materials/World/GameMaterials/MI_Highlight.MI_Highlight" :!class /Script/Engine.MeshComponent)))

(fn ReturnInteractStatus
  (return (and (Variables|Default|GetIsInteractable) (not (Variables|Default|GetSolved))) "NewEnumerator7"))

(fn ReturnSolvedStatus
  (return (Variables|Default|GetSolved)))