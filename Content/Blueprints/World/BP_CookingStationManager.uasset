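; BP_CookingStationManager runs a cooking puzzle in which ingredients must be used in recipe order, then finished at the pot.
; It binds to the cooking view, recipe book, ingredients and pot, handing possession between view and magic book and tracking recipe progress.
; Wrong inputs reset progress, while a correct pot use sends a React message to that recipe's ability manager.
; Its own React event raises the recipe book's recipe limit.
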(event Custom|ViewInteract
  (params (HitActor :type Actor%20Object%20Reference) (Player :type BP%20Player%20Object%20Reference) (CameraTransform :type Transform))
  (if (== (Utilities|GetClass HitActor) "/Game/Blueprints/World/BP_MagicBook.BP_MagicBook_C")
    (Default|Possess (Variables|Default|GetRecipeBook) CameraTransform)
    (Variables|/Game/Blueprints/World/BP_CookingView.BP_CookingView_C|SetIsPossessed (Variables|Default|GetCookingView) false)
    (else
      (Class|BPIInteract|Interact(Message) HitActor Player))))

(event Custom|BookUnpossess
  (bind _returnvalue (Game|GetPlayerController 0))
  (Variables|/Game/Blueprints/World/BP_CookingView.BP_CookingView_C|SetIsPossessed (Variables|Default|GetCookingView) true)
  (Pawn|Possess _returnvalue (Variables|Default|GetCookingView))
  (Pawn|SetControlRotation _returnvalue (.Rotation (Math|Transform|BreakTransform (stale Custom|ViewInteract CameraTransform)))))

(event Custom|NewRecepiIndex
  (params (RecipeIndex :type Integer))
  (if (not (== RecipeIndex (Variables|Default|GetCurrentRecepiIndex)))
    (Variables|Default|SetCurrentRecepiIndex RecipeIndex)
    (Variables|Default|SetRecipeProgress 0)
    (Audio|PlaySound2D "/Game/Audio/SoundSources/DropInCauldron.DropInCauldron" 1.0 1.0 0.0 0 0)))

(event Custom|IngridientUsed
  (params (UsedIngridient :type E_MagicIngredience%20Enum :default "NewEnumerator0"))
  (if (Utilities|Enum|Equal(Enum) UsedIngridient (Utilities|Array|Get(acopy) (Utilities|Struct|BreakStruct_MagicRecipes (Utilities|Array|Get(acopy) (Variables|Default|GetRecepis) (Variables|Default|GetCurrentRecepiIndex))) (Variables|Default|GetRecipeProgress)))
    (Math|Integer|IncrementInt (Variables|Default|GetRecipeProgress)
      (:%20%20
        (Audio|PlaySound2D "/Game/Audio/SoundSources/PuzzlePositive.PuzzlePositive" 1.0 1.0 0.0 0 0)
        (Development|PrintString "Right ingriedient")))
    (else
      (Default|CallIngredientFail)
      (Variables|Default|SetRecipeProgress 0)
      (Audio|PlaySound2D "/Game/Audio/SoundSources/PuzzleNegativeSound.PuzzleNegativeSound" 1.0 1.0 0.0 0 0)
      (Development|PrintString "wrong ingriedient"))))

(event Custom|PotUsed
  (if (== (Variables|Default|GetRecipeProgress) (+ (Utilities|Array|LastIndex (Utilities|Struct|BreakStruct_MagicRecipes (Utilities|Array|Get(acopy) (Variables|Default|GetRecepis) (Variables|Default|GetCurrentRecepiIndex)))) 1))
    (Default|CallPotSuccess)
    (Class|BPIReact|React(Message) (.Value (Utilities|Map|Find (Variables|Default|GetAbilityManagers) (Variables|Default|GetCurrentRecepiIndex))) true)
    (Variables|Default|SetRecipeProgress 0)
    (Audio|PlaySound2D "/Game/Audio/SoundSources/DropInCauldron.DropInCauldron" 1.0 1.0 0.0 0 0)
    (Development|PrintString "correct Pot")
    (else
      (Variables|Default|SetRecipeProgress 0)
      (Audio|PlaySound2D "/Game/Audio/SoundSources/PuzzleNegativeSound.PuzzleNegativeSound" 1.0 1.0 0.0 0 0)
      (Development|PrintString "incorrect pot"))))

(event EventBeginPlay
  (Utilities|FlowControl|Sequence
    (:then_0
      (bind _output_get (Variables|Default|SetCurrentRecepiIndex (Variables|Default|GetStartingRecepiIndex)))
      (Default|StartingRecepi (Variables|Default|GetRecipeBook) _output_get))
    (:then_1
      (EventDispatchers|BindEventtoInteract (Variables|Default|GetCookingView) (EventDispatchers|CreateEvent :!event Custom|ViewInteract))
      (EventDispatchers|BindEventtoPossessionLost (Variables|Default|GetRecipeBook) (EventDispatchers|CreateEvent :!event Custom|BookUnpossess))
      (EventDispatchers|BindEventtoNewRecipetoUse (Variables|Default|GetRecipeBook) (EventDispatchers|CreateEvent :!event Custom|NewRecepiIndex))
      (EventDispatchers|BindEventtoIngridientUsed (Variables|Default|GetIngredience) (EventDispatchers|CreateEvent :!event Custom|IngridientUsed))
      (EventDispatchers|BindEventtoCookingPotUsed (Variables|Default|GetPot) (EventDispatchers|CreateEvent :!event Potused)))))

(event EventReact
  (params (Solved :type Boolean))
  (Default|IncreaseRecepiLimit (Variables|Default|GetRecipeBook)))

(fn ConstructionScript)

(fn ReturnSolvedStatus
  (return true))