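; BP_Collectable is a world item that the player picks up into an inventory through interaction.
; Interact snaps it to the player's InventoryScene, turns off mesh collision and shadow, adds it to the inventory and calls OnCollected.
; EnableCollision restores collision and shadow casting.
; A settable IsInteractable flag is reported by ReturnInteractStatus along with a fixed interaction type.
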(event Custom|EnableCollision
  (Collision|SetCollisionEnabled (Variables|Default|GetMesh) "QueryAndPhysics")
  (Rendering|SetCastShadow (Variables|Default|GetMesh) true))

(event EventSetInteractStatus
  (params (NewInteractStatus :type Boolean))
  (Variables|Default|SetIsInteractable NewInteractStatus))

(event EventInteract
  (params (Player :type BP%20Player%20Object%20Reference))
  (Transformation|AttachComponentToComponent (Variables|/Game/Blueprints/Core/BP_Player.BP_Player_C|GetInventoryScene Player) "None" "SnapToTarget" "SnapToTarget" "SnapToTarget" true)
  (Collision|SetCollisionEnabled (Variables|Default|GetMesh) "NoCollision")
  (Rendering|SetCastShadow (Variables|Default|GetMesh) false)
  (Default|AddtoInventory Player self)
  (Default|CallOnCollected))

(fn ConstructionScript)

(fn ReturnInteractStatus
  (return (Variables|Default|GetIsInteractable) "NewEnumerator1"))