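; Inspectable world object that the player possesses on interact to examine and rotate up close.
; Its camera snaps to the player's view while MoveComponentTo eases the object in front of it, then an inspect widget is added to the main stack.
; Look input rotates the mesh by re-attaching it between separate yaw and pitch pivot components.
; Interacting again removes the widget, eases everything back and restores player possession and control rotation.
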(event Custom|MoveInspectable
  (params (OnPosses :type Boolean))
  (bind _defaulttransform (Variables|Default|GetDefaultTransform))
  (bind _meshtransform (Variables|Default|GetmeshTransform))
  (bind _camera (Variables|Default|GetCamera))
  (bind _camredistance (Variables|Default|GetCamreDistance))
  (bind _returnvalue (Math|Vector|GetForwardVector _camera))
  (bind _relativelocation (Variables|/Script/Engine.SceneComponent|GetRelativeLocation _camera))
  (bind _relativerotation (Variables|/Script/Engine.SceneComponent|GetRelativeRotation _camera))
  (bind _returnvalue_2 (* _returnvalue _camredistance))
  (bind _returnvalue_3 (+ _relativelocation _returnvalue_2))
  (bind _returnvalue_4 (Math|Transform|MakeTransform _returnvalue_3 _relativerotation))
  (bind _returnvalue_5 (Math|Transform|SelectTransform _returnvalue_4 _defaulttransform OnPosses))
  (bind (_location _rotation) (Math|Transform|BreakTransform _returnvalue_5))
  (Utilities|FlowControl|Sequence
    (:then_0
      (Components|MoveComponentTo (Variables|Default|GetRotationScene) _location _rotation true true (Variables|Default|GetPossesDuration) true))
    (:then_1
      (Transformation|AttachComponentToComponent (Variables|Default|GetMesh) (Variables|Default|GetRotationScene) "None" "KeepWorld" "KeepWorld" "KeepWorld" true)
      (Components|MoveComponentTo (Variables|Default|GetMesh) (.location _meshtransform) (.rotation _meshtransform) true true (Variables|Default|GetPossesDuration) true)
      (bind _output_get (Variables|Default|SetCanRotate OnPosses))
      (if _output_get
        (bind _returnvalue_6 (Class|CommonActivatableWidgetContainerBase|AddWidget (CallFunction|ReturnMainStack (Game|GetPlayerController 0)) "/Game/Blueprints/UI/CAW_Inspect.CAW_Inspect_C"))
        (Variables|Default|SetWidget _returnvalue_6)
        (else
          (Pawn|Possess (Game|GetPlayerController 0) (Variables|Default|GetPlayerRef))
          (Pawn|SetControlRotation (Game|GetPlayerController 0) (Variables|Default|GetControlRotation)))))))

(event Input|EnhancedActionEvents|EnhancedInputActionIA_Interact
  (params (ActionValue :type Boolean) (ElapsedSeconds :type Float%20%28double-precision%29) (TriggeredSeconds :type Float%20%28double-precision%29) (InputAction :type Input%20Action%20Object%20Reference :default "/Game/Inputs/IA_Interact.IA_Interact"))
  (:Started
    (Variables|Default|GetCanRotate
      (:then
        (Variables|Default|SetCanRotate false)
        (Utilities|FlowControl|DelayUntilNextTick)
        (Class|CommonActivatableWidgetContainerBase|RemoveWidget (CallFunction|ReturnMainStack (Game|GetPlayerController 0)) (Variables|Default|GetWidget))
        (CallFunction|MoveInspectable false))
      (:else))))

(event Input|EnhancedActionEvents|EnhancedInputActionIA_Look
  (params (ActionValue :type Vector%202D%20Structure) (ElapsedSeconds :type Float%20%28double-precision%29) (TriggeredSeconds :type Float%20%28double-precision%29) (InputAction :type Input%20Action%20Object%20Reference :default "/Game/Inputs/IA_Look.IA_Look"))
  (bind (_x _y) (Math|Vector2D|BreakVector2D ActionValue))
  (if (Variables|Default|GetCanRotate)
    (Transformation|AttachComponentToComponent (Variables|Default|GetMesh) (Variables|Default|GetXScene) "None" "KeepWorld" "KeepWorld" "KeepWorld" true)
    (Transformation|AddLocalRotation (Variables|Default|GetXScene) (Math|Rotator|MakeRotator 0.0 0.0 (* _x -1.0)) true false)
    (Transformation|AttachComponentToComponent (Variables|Default|GetMesh) (Variables|Default|GetYScene) "None" "KeepWorld" "KeepWorld" "KeepWorld" true)
    (Transformation|AddLocalRotation (Variables|Default|GetYScene) (Math|Rotator|MakeRotator 0.0 _y 0.0) true false)))

(event EventSetInteractStatus
  (params (NewInteractStatus :type Boolean))
  (Variables|Default|SetIsInteractable NewInteractStatus))

(event EventInteract
  (params (Player :type BP%20Player%20Object%20Reference))
  (bind _output_get (Variables|Default|SetPlayerRef Player))
  (Variables|Default|SetControlRotation (Pawn|GetControlRotation _output_get :!class /Script/Engine.Pawn))
  (Transformation|SetWorldTransform (Variables|Default|GetCamera) (Transformation|GetWorldTransform (Variables|/Game/Blueprints/Core/BP_Player.BP_Player_C|GetCamera (Variables|Default|GetPlayerRef))) false true)
  (Pawn|Possess (Game|GetPlayerController 0) self)
  (CallFunction|MoveInspectable true))

(event EventBeginPlay
  (Variables|Default|SetDefaultTransform (Transformation|GetRelativeTransform (Variables|Default|GetRotationScene)))
  (Variables|Default|SetmeshTransform (Transformation|GetRelativeTransform (Variables|Default|GetMesh))))

(fn ConstructionScript)

(fn ReturnInteractStatus
  (return (Variables|Default|GetIsInteractable) "NewEnumerator3"))