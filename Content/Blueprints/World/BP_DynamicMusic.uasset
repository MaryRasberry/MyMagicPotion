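; Dynamic music actor that spawns a 2D sound on BeginPlay and adjusts its OverallGain parameter as React receives solved or unsolved states.
; A Gain counter holds the level, and GainTimeline blends one step up when solved or down when unsolved.
; React polls each tick while the timeline plays, delaying new changes until it finishes.
; ReturnSolvedStatus always returns false.
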(event EventBeginPlay
  (bind _returnvalue (Audio|SpawnSound2D (Variables|Default|GetMusicIsPlaying) 1.0 1.0 0.0 0))
  (Variables|Default|SetMusic _returnvalue))

(event EventReact
  (params (Solved :type Boolean))
  (if (Audio|Components|Audio|IsPlaying (Variables|Default|GetGainTimeline)) :!label _label
    (Utilities|FlowControl|DelayUntilNextTick)
    (goto _label)
    (elif Solved
      (bind (_direction _gain) (Timeline|GainTimeline PlayFromStart)
        (:Update
          (Audio|Parameter|SetFloatParameter (Variables|Default|GetMusic) "OverallGain" (+ _gain (Variables|Default|GetGain)) :!class /Script/Engine.AudioComponent))
        (:Finished
          (switch Utilities|FlowControl|Switch|SwitchonETimelineDirection _direction
            (:Forward
              (bind _result (Math|Float|IncrementFloat (Variables|Default|GetGain))
                (:%20%20
                  (Audio|Parameter|SetFloatParameter (Variables|Default|GetMusic) "OverallGain" _result :!class /Script/Engine.AudioComponent)))))))
      (else
        (Math|Float|DecrementFloat (Variables|Default|GetGain)
          (:%20%20
            (Timeline|GainTimeline ReverseFromEnd)))))))

(fn ConstructionScript)

(fn ReturnSolvedStatus
  (return false))