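; Game instance that owns the player's settings save and a show-credits flag, with getters for both.
; On init it loads the settings save, or creates one and applies default graphics, VSync and frame-rate settings.
; It retries each tick until a GameMode is valid, then applies saved sound-class volumes through a sound mix and sets color vision deficiency correction.
; Shutdown writes the settings back to the save slot.
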(event EventInit
  (bind _returnvalue (SaveGame|DoesSaveGameExist (Variables|Default|GetSaveGameSlotName)))
  (if _returnvalue
    (bind _returnvalue_2 (SaveGame|LoadGamefromSlot (Variables|Default|GetSaveGameSlotName)))
    (bind _asbp_settings_save (Utilities|Casting|CastToBP_SettingsSave _returnvalue_2))
    (Variables|Default|SetSaveGameRef _asbp_settings_save)
    (else
      (bind _returnvalue_3 (SaveGame|CreateSaveGameObject "/Game/Blueprints/Core/BP_SettingsSave.BP_SettingsSave_C"))
      (Variables|Default|SetSaveGameRef _returnvalue_3)
      (bind _returnvalue_4 (Settings|GetGameUserSettings))
      (Class|GameUserSettings|SetVSyncEnabled _returnvalue_4 false)
      (Class|GameUserSettings|SetFrameRateLimit _returnvalue_4 9e+01)
      (Class|GameUserSettings|SetShadowQuality _returnvalue_4 1)
      (Class|GameUserSettings|SetGlobalIlluminationQuality _returnvalue_4 2)
      (Class|GameUserSettings|ApplySettings _returnvalue_4 true)))
  (Utilities|IsValid (Game|GetGameMode) :!label _label
    (:Is%20Valid
      (Audio|SetSoundMixClassOverride "/Game/Audio/SCM_Main.SCM_Main" "/Game/Audio/SC_Master.SC_Master" (Variables|/Game/Blueprints/Core/BP_SettingsSave.BP_SettingsSave_C|GetMasterVolume (Variables|Default|GetSaveGameRef)) 1.0 0.0 true)
      (Audio|SetSoundMixClassOverride "/Game/Audio/SCM_Main.SCM_Main" "/Game/Audio/SC_Music.SC_Music" (Variables|/Game/Blueprints/Core/BP_SettingsSave.BP_SettingsSave_C|GetMusicVolume (Variables|Default|GetSaveGameRef)) 1.0 0.0 true)
      (Audio|SetSoundMixClassOverride "/Game/Audio/SCM_Main.SCM_Main" "/Game/Audio/SC_SFX.SC_SFX" (Variables|/Game/Blueprints/Core/BP_SettingsSave.BP_SettingsSave_C|GetSfxVolume (Variables|Default|GetSaveGameRef)) 1.0 0.0 true)
      (Audio|SetSoundMixClassOverride "/Game/Audio/SCM_Main.SCM_Main" "/Game/Audio/SC_Atmo.SC_Atmo" (Variables|/Game/Blueprints/Core/BP_SettingsSave.BP_SettingsSave_C|GetAtmoVolume (Variables|Default|GetSaveGameRef)) 1.0 0.0 true)
      (Audio|PushSoundMixModifier "/Game/Audio/SCM_Main.SCM_Main")
      (Class|WidgetBlueprintLibrary|SetColorVisionDeficiencyType (Variables|/Game/Blueprints/Core/BP_SettingsSave.BP_SettingsSave_C|GetColorDef (Variables|Default|GetSaveGameRef)) 1.0 true))
    (:Is%20Not%20Valid
      (Utilities|FlowControl|DelayUntilNextTick)
      (goto _label))))

(event EventShutdown
  (SaveGame|SaveGametoSlot (Variables|Default|GetSaveGameRef) (Variables|Default|GetSaveGameSlotName)))

(event EventSetShowCredits
  (params (Show :type Boolean))
  (Variables|Default|SetShowCredits Show))

(fn ReturnSaveGame
  (return (Variables|Default|GetSaveGameRef)))

(fn ReturnShowCredits
  (return (Variables|Default|GetShowCredits)))