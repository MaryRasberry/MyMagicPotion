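; First-person player character handling gated movement and look input, surface-based footsteps, interaction and a cyclable held-item inventory.
; A looping timer traces from the camera to set the current BPI_Interact target, driving a crosshair material parameter and notifying listeners.
; CookingInteract reuses that check with an external trace for when the player is unpossessed.
; Inventory changes and next/previous input refresh which item is visible; look sensitivity comes from saved settings.
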(event EventBeginPlay
  (Utilities|Time|SetTimerbyFunctionName 0 "InteractCheck" 0.1 true true)
  (Components|Timeline|SetPlayRate (Variables|Default|GetCrosshairTimeline) (|(1/{ADE3FB85-49F7-E4D1-910D-EBBC1CD90F85})))
  (bind _settingssave (Class|BPIGameInstance|ReturnSaveGame(Message) (Game|GetGameInstance)))
  (bind _output_get (Variables|Default|SetSettingsSave _settingssave))
  (Variables|Default|SetCurrentLookSensivity (Variables|/Game/Blueprints/Core/BP_SettingsSave.BP_SettingsSave_C|GetLookSensivity _output_get))
  (Audio|Components|Audio|Play (Variables|Default|GetFootStepTimeline)))

(fn ConstructionScript)

(event Input|EnhancedActionEvents|EnhancedInputActionIA_Look
  (params (ActionValue :type Vector%202D%20Structure) (ElapsedSeconds :type Float%20%28double-precision%29) (TriggeredSeconds :type Float%20%28double-precision%29) (InputAction :type Input%20Action%20Object%20Reference :default "/Game/Inputs/IA_Look.IA_Look"))
  (bind (_x _y) (Math|Vector2D|BreakVector2D ActionValue))
  (bind _currentlooksensivity (Variables|Default|GetCurrentLookSensivity))
  (Utilities|HasInput
    (:true
      (Pawn|Input|AddControllerYawInput (* _currentlooksensivity _x))
      (Pawn|Input|AddControllerPitchInput (* _currentlooksensivity _y)))))

(event Input|EnhancedActionEvents|EnhancedInputActionIA_Move
  (params (ActionValue :type Vector%202D%20Structure) (ElapsedSeconds :type Float%20%28double-precision%29) (TriggeredSeconds :type Float%20%28double-precision%29) (InputAction :type Input%20Action%20Object%20Reference :default "/Game/Inputs/IA_Move.IA_Move"))
  (bind (_x _y) (Math|Vector2D|BreakVector2D ActionValue))
  (Utilities|HasInput
    (:true
      (Pawn|Input|AddMovementInput (Transformation|GetActorRightVector) _x false)
      (Pawn|Input|AddMovementInput (Transformation|GetActorForwardVector) _y false))))

(event Input|EnhancedActionEvents|EnhancedInputActionIA_Jump
  (params (ActionValue :type Boolean) (ElapsedSeconds :type Float%20%28double-precision%29) (TriggeredSeconds :type Float%20%28double-precision%29) (InputAction :type Input%20Action%20Object%20Reference :default "/Game/Inputs/IA_Jump.IA_Jump"))
  (:Started
    (Utilities|HasInput
      (:true
        (Character|Jump))))
  (:Completed
    (Character|StopJumping)))

(event Custom|InteractCheck
  (bind _ispossessed (Variables|Default|GetIsPossessed))
  (bind _camera (Variables|Default|GetCamera))
  (bind _ispossessed_2 (Variables|Default|GetIsPossessed))
  (bind _returnvalue (Transformation|GetWorldLocation _camera))
  (bind (_outhit _returnvalue_2) (Collision|LineTraceByChannel _returnvalue (+ _returnvalue (* (Math|Vector|GetForwardVector _camera) (Variables|Default|GetInteractDistance))) "TraceTypeQuery1" false 0 "None"))
  (if (select _ispossessed_2 _returnvalue_2 (stale Custom|CookingInteract TraceReturn))
    (bind (_isinteractable _type) (Class|BPIInteract|ReturnInteractStatus(Message) (.HitActor (Collision|BreakHitResult (select _ispossessed_2 _outhit (stale Custom|CookingInteract TraceResult))))))
    (Default|CallOnInteractionChecked _type (and _isinteractable (Utilities|DoesObjectImplementInterface (.HitActor (Collision|BreakHitResult (select _ispossessed_2 _outhit (stale Custom|CookingInteract TraceResult)))) "/Game/Blueprints/Interfaces/BPI_Interact.BPI_Interact_C")))
    (if (and _isinteractable (Utilities|DoesObjectImplementInterface (.HitActor (Collision|BreakHitResult (select _ispossessed_2 _outhit (stale Custom|CookingInteract TraceResult)))) "/Game/Blueprints/Interfaces/BPI_Interact.BPI_Interact_C"))
      (if _ispossessed
        (Variables|Default|SetCurrentInteractable (.HitActor (Collision|BreakHitResult (select _ispossessed_2 _outhit (stale Custom|CookingInteract TraceResult)))))
        (bind _value (Timeline|CrosshairTimeline Play)
          (:Update
            (Rendering|Material|SetScalarParameterValue "/Game/Materials/UI/MPC_Player.MPC_Player" "LookAt" _value :!class /Script/Engine.KismetMaterialLibrary)))
        (else
          (Variables|Default|SetCurrentInteractable 0)
          (Timeline|CrosshairTimeline Play)))
      (else
        (if _ispossessed :!label _label
          _
          (else
            _))
        (Variables|Default|SetCurrentInteractable 0)
        (Timeline|CrosshairTimeline Reverse)))
    (else
      (Default|CallOnInteractionChecked "NewEnumerator0" false)
      (goto _label))))

(event Custom|CookingInteract
  (params (TraceReturn :type Boolean) (TraceResult :type Hit%20Result%20Structure%20%28by%20ref%29))
  (bind _ispossessed (Variables|Default|GetIsPossessed))
  (bind _ispossessed_2 (Variables|Default|GetIsPossessed))
  (if (select _ispossessed_2 (stale Custom|InteractCheck _returnvalue_2) TraceReturn)
    (bind (_isinteractable _type) (Class|BPIInteract|ReturnInteractStatus(Message) (.HitActor (Collision|BreakHitResult (select _ispossessed_2 (stale Custom|InteractCheck _outhit) TraceResult)))))
    (Default|CallOnInteractionChecked _type (and _isinteractable (Utilities|DoesObjectImplementInterface (.HitActor (Collision|BreakHitResult (select _ispossessed_2 (stale Custom|InteractCheck _outhit) TraceResult))) "/Game/Blueprints/Interfaces/BPI_Interact.BPI_Interact_C")))
    (if (and _isinteractable (Utilities|DoesObjectImplementInterface (.HitActor (Collision|BreakHitResult (select _ispossessed_2 (stale Custom|InteractCheck _outhit) TraceResult))) "/Game/Blueprints/Interfaces/BPI_Interact.BPI_Interact_C"))
      (if _ispossessed
        (Variables|Default|SetCurrentInteractable (.HitActor (Collision|BreakHitResult (select _ispossessed_2 (stale Custom|InteractCheck _outhit) TraceResult))))
        (bind _value (Timeline|CrosshairTimeline Play)
          (:Update
            (Rendering|Material|SetScalarParameterValue "/Game/Materials/UI/MPC_Player.MPC_Player" "LookAt" _value :!class /Script/Engine.KismetMaterialLibrary)))
        (else
          (Variables|Default|SetCurrentInteractable 0)
          (Timeline|CrosshairTimeline Play)))
      (else
        (if _ispossessed :!label _label
          _
          (else
            _))
        (Variables|Default|SetCurrentInteractable 0)
        (Timeline|CrosshairTimeline Reverse)))
    (else
      (Default|CallOnInteractionChecked "NewEnumerator0" false)
      (goto _label))))

(event Input|EnhancedActionEvents|EnhancedInputActionIA_Interact
  (params (ActionValue :type Boolean) (ElapsedSeconds :type Float%20%28double-precision%29) (TriggeredSeconds :type Float%20%28double-precision%29) (InputAction :type Input%20Action%20Object%20Reference :default "/Game/Inputs/IA_Interact.IA_Interact"))
  (:Started
    (Utilities|HasInput
      (:true
        (bind _currentinteractable (Variables|Default|GetCurrentInteractable)
          (:then
            (Class|BPIInteract|Interact(Message) _currentinteractable self))
          (:else))))))

(event Custom|AddToInventory
  (params (CollectableToAdd :type BP%20Collectable%20Object%20Reference%20%28by%20ref%29))
  (bind _returnvalue (Utilities|Array|Add (Variables|Default|GetInvventory) CollectableToAdd))
  (CallFunction|RefreshInventory _returnvalue))

(event Custom|RefreshInventory
  (params (NewInventoryIndex :type Integer))
  (Variables|Default|SetInventoryIndex NewInventoryIndex)
  (for (_array_element _array_index) (Variables|Default|GetInvventory)
    (if (!= _array_index 0)
      (Rendering|SetActorHiddenInGame _array_element (!= _array_index (Variables|Default|GetInventoryIndex))))))

(event Custom|RemoveFromInventory
  (params (CollectableToMove :type BP%20Collectable%20Object%20Reference%20%28by%20ref%29) (ShouldDestroy :type Boolean))
  (Utilities|Array|RemoveItem (Variables|Default|GetInvventory) CollectableToMove)
  (CallFunction|RefreshInventory (- (Variables|Default|GetInventoryIndex) 1))
  (if ShouldDestroy
    (Actor|DestroyActor CollectableToMove)))

(event Input|EnhancedActionEvents|EnhancedInputActionIA_NextItem
  (params (ActionValue :type Boolean) (ElapsedSeconds :type Float%20%28double-precision%29) (TriggeredSeconds :type Float%20%28double-precision%29) (InputAction :type Input%20Action%20Object%20Reference :default "/Game/Inputs/IA_NextItem.IA_NextItem"))
  (bind _inventoryindex (Variables|Default|GetInventoryIndex))
  (bind _returnvalue (+ _inventoryindex 1))
  (:Started
    (CallFunction|RefreshInventory (Math|Integer|SelectInt 0 _returnvalue (> _returnvalue (Utilities|Array|LastIndex (Variables|Default|GetInvventory)))))))

(event Input|EnhancedActionEvents|EnhancedInputActionIA_PreviousItem
  (params (ActionValue :type Boolean) (ElapsedSeconds :type Float%20%28double-precision%29) (TriggeredSeconds :type Float%20%28double-precision%29) (InputAction :type Input%20Action%20Object%20Reference :default "/Game/Inputs/IA_PreviousItem.IA_PreviousItem"))
  (bind _inventoryindex (Variables|Default|GetInventoryIndex))
  (bind _returnvalue (- _inventoryindex 1))
  (:Started
    (CallFunction|RefreshInventory (Math|Integer|SelectInt (Utilities|Array|LastIndex (Variables|Default|GetInvventory)) _returnvalue (< _returnvalue 0)))))